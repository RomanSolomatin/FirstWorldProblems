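; Credit card pickup actor that the player collects into the inventory.
; On BeginPlay it creates a pickup text widget, fills in its item struct with itself, and binds to the player character's pickup event.
; When that event fires and the character's current item is this actor, it adds the item to the HUD inventory, removes the text and refreshes.
; A separate Clicked function destroys its Paper sprite.
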(event Custom|PickUpItem_Event
  (bind _mycharacter (Variables|Default|GetMyCharacter))
  (bind _gamehud (Variables|/Game/BluePrints/myCharacter.myCharacter_C|GetGameHUD _mycharacter))
  ;[1 1 1] Pick Up and Add Item to inventory
  (if (== (Variables|/Game/BluePrints/myCharacter.myCharacter_C|GetinventoryItem (Variables|Default|GetMyCharacter)) self)
    (Utilities|Array|Add (Variables|/Game/BluePrints/UMG/InGameMenu.InGameMenu_C|GetInventory _gamehud) (Variables|Default|GetItemInfo))
    (Class|UserWidget|RemovefromViewport (Variables|Default|GetPickUpTextWidget))
    (Default|RefreshInventory _gamehud)))

(event EventBeginPlay
  (bind _iteminfo (Variables|Default|GetItemInfo))
  (bind (_item _itemimage _pickuptext) (Utilities|Struct|BreakInventoryStruct _iteminfo))
  ;[1 1 1] Event Begin Play
  (bind _returnvalue (UserInterface|CreateWidget "/Game/BluePrints/UMG/PickUpText.PickUpText_C"))
  (Variables|/Game/BluePrints/UMG/PickUpText.PickUpText_C|SetPickUpActor _returnvalue _item)
  (Variables|Default|SetPickUpTextWidget _returnvalue)
  (Variables|/Game/BluePrints/UMG/PickUpText.PickUpText_C|SetPickUpText _returnvalue _pickuptext)
  (Utilities|Struct|SetmembersinInventoryStruct _iteminfo self)
  (bind _asmycharacter_c (Utilities|Casting|CastTomyCharacter (Pawn|GetControlledPawn (Game|GetPlayerController 0))))
  (Variables|Default|SetMyCharacter _asmycharacter_c)
  (EventDispatchers|BindEventtoPickUpItem _asmycharacter_c (delegate Custom|PickUpItem_Event)))

(fn ConstructionScript)

(fn Clicked
  (Components|DestroyComponent (Variables|Default|GetPaperSprite1))
  (return false))