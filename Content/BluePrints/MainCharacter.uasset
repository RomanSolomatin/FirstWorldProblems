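; Main character Blueprint that lets the player click items in the world through the PickUp input action.
; On press, it runs a complex cursor hit test limited to one custom object type and stores the hit actor in InvItem.
; It casts that actor to InventoryItem and calls ClickedMessage, with debug prints reporting the result, a failed cast or no hit.
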(event Input|ActionEvents|InputActionPickUp
  (bind _returnvalue (Game|GetPlayerController 0))
  (bind _array (Utilities|Array|MakeArray "ObjectTypeQuery7"))
  (bind (_hitresult _returnvalue_2) (Class|PlayerController|GetHitResultUnderCursorforObjects _returnvalue _array true))
  (:Pressed
    (if _returnvalue_2
      (Variables|Default|SetInvItem (.HitActor (Collision|BreakHitResult _hitresult)))
      (bind _asinventoryitem_c (Utilities|Casting|CastToInventoryItem (Variables|Default|GetInvItem))
        (:then
          (bind _issuccessful (Class|InventoryItems|Clicked(Message) _asinventoryitem_c))
          (if _issuccessful
            (Development|PrintString "Success")
            (else
              (Development|PrintString "Fail"))))
        (:CastFailed
          (Development|PrintString "Cast failed")))
      (else
        (Development|PrintString "No item")))))

(fn ConstructionScript)