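; Player character Blueprint that handles cursor-based item pickup and creates the in-game HUD.
; On BeginPlay it creates the InGameMenu widget, adds it to the viewport and keeps it as GameHUD.
; The PickUp input traces under the cursor against a custom object type and stores the hit result and actor.
; It then sends ClickedMessage to that actor and fires CallPickUpItem, without branching on whether anything was hit.
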(event EventBeginPlay
  (bind _returnvalue (UserInterface|CreateWidget "/Game/BluePrints/UMG/InGameMenu.InGameMenu_C"))
  (UserInterface|Viewport|AddtoViewport _returnvalue)
  (Variables|Default|SetGameHUD _returnvalue))

(event Input|ActionEvents|InputActionPickUp
  (bind _returnvalue (Game|GetPlayerController 0))
  (bind _array (Utilities|Array|MakeArray "ObjectTypeQuery7"))
  (bind (_hitresult _returnvalue_2) (Class|PlayerController|GetHitResultUnderCursorforObjects _returnvalue _array true))
  (:Pressed
    (Variables|Default|SetisPickUpItem _returnvalue_2)
    (Variables|Default|SetinventoryItem (.HitActor (Collision|BreakHitResult _hitresult)))
    (Class|InventoryItems|Clicked(Message) (Variables|Default|GetinventoryItem))
    (Default|CallPickUpItem)))

(fn ConstructionScript)